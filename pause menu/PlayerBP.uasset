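; Player character Blueprint with single-axis movement along world X, variable-height jumping and a pause menu on the M key.
; M creates the Pause_Menu widget once, caches it, adds it to the viewport, switches input to UI-only and pauses the game.
; The construction script sets jump velocity and hold time.
; Destruction calls Open Level with the name "None", and the colour-switch input only prints placeholder text.
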(event `InputAxis|Move(Right)`
  (params (AxisValue :type "Float (single-precision)"))
  ;[1 1 1] Movement
  (`self.AddMovementInput` (0.5 0.0 0.0) AxisValue))

(event `Key|M`
  (params (Key :type "Key Structure" :default "AnyKey"))
  (bind _referencethepausemenu (`self.ReferenceThePauseMenu`))
  ;[1 1 1] Pause Menu "M" key
  (:`Pressed`
    (`/Engine/EditorBlueprintResources/StandardMacros.IsValid` _referencethepausemenu
      (:`Is Valid`
        _)
      (:`Is Not Valid`
        (bind _returnvalue (`|CreateWidget` "/Game/Menu/Pause_Menu.Pause_Menu_C"))
        (bind _output_get (set `self.ReferenceThePauseMenu` _returnvalue))))
    (`WidgetBlueprintLibrary.SetInputMode_UIOnlyEx` (`GameplayStatics.GetPlayerController` 0) _referencethepausemenu)
    (`UserWidget.AddToViewport` _output_get 0)
    (`GameplayStatics.SetGamePaused` true)))

(event `self.ReceiveDestroyed`
  ;[1 1 1] Pause Menu "M" key
  (`GameplayStatics.OpenLevel` "None"))

(event `InputAction|Jump`
  (params (Key :type "Key Structure" :default "AnyKey"))
  ;[1 1 1] Jumping
  (:`Pressed`
    (`self.Jump`))
  (:`Released`
    (`self.StopJumping`)))

(event `InputAction|Switching Colours`
  (params (Key :type "Key Structure" :default "AnyKey"))
  ;[1 1 1] Pause Menu "M" key
  (:`Released`
    (`KismetSystemLibrary.PrintText` "Hello")))

(fn `UserConstructionScript`
  (set `CharacterMovementComponent.JumpZVelocity` 300.0 (`self.CharacterMovement`))
  (set `self.JumpMaxHoldTime` 0.3))